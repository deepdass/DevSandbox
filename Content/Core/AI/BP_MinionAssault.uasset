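; Assault minion AI character that shows damage popups on health loss and can be sliced in half by a sawblade.
; Slice forwards to ServerSliceEffect, which applies lethal damage and fakes the cut by hiding opposite bones on two meshes.
; It also sets the second mesh's ragdoll collision profile, launches it and sprays Niagara blood along the blade's velocity.
; SetCurrentScale forwards shrink/grow scale through a server event to ACShrinkGrowActor.
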(event OnHealthChanged(AttributeComp)
  (params (InstigatorActor :type Actor%20Object%20Reference) (OwningComp :type S%20Attribute%20Component%20Object%20Reference) (Health :type Float%20%28single-precision%29) (Delta :type Float%20%28single-precision%29))
  (if (< Delta 0.0)
    (bind _returnvalue (UserInterface|CreateWidget "/Game/Core/UI/WorldWidget/WBP_DamagePopup.WBP_DamagePopup_C" 0 self (Math|Float|Absolute(Float) Delta)))
    (UserInterface|Viewport|AddtoViewport _returnvalue 0)))

(event Custom|ServerSliceEffect
  (params (ServerSawblade :type Scene%20Component%20Object%20Reference))
  (bind _charactermeshother (Variables|Default|GetCharacterMeshOther))
  (bind _attributecomp (Variables|Default|GetAttributeComp))
  (Development|SetHiddeninGame (Variables|Default|GetCharacterMeshOther) false false)
  (Class|SAttributeComponent|ApplyHealthChange _attributecomp 0 (* (Class|SAttributeComponent|GetMaxHealth _attributecomp) -1.0))
  (Components|SkinnedMesh|HideBonebyName (Variables|Character|GetMesh) "spine_02" "PBO_None")
  (Components|SkinnedMesh|HideBonebyName _charactermeshother "thigh_l" "PBO_None")
  (Components|SkinnedMesh|HideBonebyName _charactermeshother "thigh_r" "PBO_None")
  (Collision|SetCollisionProfileName _charactermeshother "Ragdoll" true :!class /Script/Engine.PrimitiveComponent)
  (Physics|AddImpulse _charactermeshother "600.000000,600.000000,12000.000000" "None" true)
  (Collision|SetCollisionResponsetoChannel _charactermeshother "ECC_Visibility" "ECR_Block")
  (Niagara|SpawnSystematLocation "/Game/Core/VFX/Blood/NS_Blood.NS_Blood" (Transformation|GetSocketLocation (Variables|Character|GetMesh) "spine_01") (Math|Rotator|MakeRotfromZ (Transformation|GetComponentVelocity ServerSawblade))))

(event Custom|ServerSetCurrentScale
  (params (ServerCurrentScale :type Vector))
  (Variables|/Game/Core/ShrinkGrow/AC_ShrinkGrowActor.AC_ShrinkGrowActor_C|SetCurrentScale (Variables|Default|GetAC_ShrinkGrowActor) ServerCurrentScale))

(event EventBeginPlay)

(event EventSetCurrentScale
  (params (ActorCurrentScale :type Vector :default "0, 0, 0"))
  (CallFunction|ServerSetCurrentScale ActorCurrentScale))

(event Collision|EventActorBeginOverlap
  (params (OtherActor :type Actor%20Object%20Reference)))

(event EventSlice
  (params (SawMesh :type Scene%20Component%20Object%20Reference))
  (CallFunction|ServerSliceEffect SawMesh))

(fn ConstructionScript)