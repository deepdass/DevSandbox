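; BP_RangedMinion is a ranged minion Blueprint that displays damage popups when it loses health.
; It listens to its attribute component's health-change event and, for negative deltas, creates a damage popup widget attached to itself showing the absolute amount.
; The graph holds no attack or movement logic, only this feedback and a disconnected debug print of an AI Blackboard object.
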(event OnHealthChanged(AttributeComp)
  (params (InstigatorActor :type Actor%20Object%20Reference) (OwningComp :type S%20Attribute%20Component%20Object%20Reference) (Health :type Float%20%28single-precision%29) (Delta :type Float%20%28single-precision%29))
  (if (< Delta 0.0)
    (bind _returnvalue (UserInterface|CreateWidget "/Game/Core/UI/WorldWidget/WBP_DamagePopup.WBP_DamagePopup_C" 0 self (Math|Float|Absolute(Float) Delta)))
    (UserInterface|Viewport|AddtoViewport _returnvalue 0)))

(event EventBeginPlay)

(event Collision|EventActorBeginOverlap
  (params (OtherActor :type Actor%20Object%20Reference)))

(event EventTick
  (params (DeltaSeconds :type Float%20%28single-precision%29)))

(fn ConstructionScript)