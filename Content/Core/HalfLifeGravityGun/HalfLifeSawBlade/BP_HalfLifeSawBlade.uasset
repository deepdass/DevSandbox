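; Half-Life style saw blade for the gravity gun that slices actors it overlaps after being pushed.
; On push it locks the constraint's swing axes, spins around its up vector, ignores Pawn collision and becomes active.
; While held it frees the swing, blocks Pawns and turns inactive.
; When active, Box overlaps send SliceMessage with the blade mesh to the other actor, leaving the slicing to that actor.
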(event OnComponentBeginOverlap(Box)
  (params (OverlappedComponent :type Primitive%20Component%20Object%20Reference) (OtherActor :type Actor%20Object%20Reference) (OtherComp :type Primitive%20Component%20Object%20Reference) (OtherBodyIndex :type Integer) (bFromSweep :type Boolean) (SweepResult :type Hit%20Result%20Structure%20%28by%20ref%29))
  (if (Variables|Default|GetIsActive)
    (Utilities|IsValid OtherActor
      (:Is%20Valid
        (Class|BPISliceableObject|Slice(Message) OtherActor (Variables|Default|GetBaseMesh))))))

(event EventBeginPlay)

(event Collision|EventActorBeginOverlap
  (params (OtherActor :type Actor%20Object%20Reference)))

(event EventTick
  (params (DeltaSeconds :type Float%20%28single-precision%29)))

(event EventOnPushObject
  (bind _physicsconstraint (Variables|Default|GetPhysicsConstraint))
  (Class|PhysicsConstraintComponent|SetAngularSwing1Limit _physicsconstraint "ACM_Locked" 0.0)
  (Class|PhysicsConstraintComponent|SetAngularSwing2Limit _physicsconstraint "ACM_Locked" 0.0)
  (Class|PrimitiveComponent|AddAngularImpulseinDegrees (Variables|Default|GetBaseMesh) (* (Math|Vector|GetUpVector (Variables|Default|GetBaseMesh)) 3.6e+03) "None" true)
  (Variables|Default|SetIsActive true)
  (Collision|SetCollisionResponsetoChannel (Variables|Default|GetBaseMesh) "ECC_Pawn" "ECR_Ignore"))

(event EventHoldingObject
  (Variables|Default|SetIsActive false)
  (Class|PhysicsConstraintComponent|SetAngularSwing1Limit (Variables|Default|GetPhysicsConstraint) "ACM_Free" 0.0)
  (Class|PhysicsConstraintComponent|SetAngularSwing2Limit (Variables|Default|GetPhysicsConstraint) "ACM_Free" 0.0)
  (Collision|SetCollisionResponsetoChannel (Variables|Default|GetBaseMesh) "ECC_Pawn" "ECR_Block"))

(fn ConstructionScript)