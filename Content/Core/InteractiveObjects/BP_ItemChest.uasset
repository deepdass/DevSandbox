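; BP_ItemChest is an interactive chest that plays a Niagara effect when its lid is opened.
; On Interact it waits briefly, runs the parent's Interact logic, then activates the effect if LidOpened is true.
; A keycard check against the instigator's SActionComponent gameplay tags, printing the missing tag, is present but disconnected and never runs.
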(event EventBeginPlay)

(event Collision|EventActorBeginOverlap
  (params (OtherActor :type Actor%20Object%20Reference)))

(event EventTick
  (params (DeltaSeconds :type Float%20%28single-precision%29)))

(event EventInteract
  (params (InstigatorPawn :type Pawn%20Object%20Reference))
  (Utilities|FlowControl|Delay 0.25)
  (|CallParentFunction InstigatorPawn)
  (if (Variables|Default|GetbLidOpened)
    (Components|Activation|Activate (Variables|Default|GetNiagara) false)))

(fn ConstructionScript)