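; BP_Enemy is an enemy character that can be sliced in half at the waist by a sawblade and have its shrink/grow scale set.
; Slice forwards to a Server event that switches to ragdoll collision and fakes the cut by hiding opposite bones on two overlapping meshes.
; It launches the second mesh with an impulse and spawns Niagara blood oriented along the blade's velocity.
; SetCurrentScale likewise forwards the scale to ACShrinkGrowActor.
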(event Custom|ServerSliceEffect
  (params (ServerSawblade :type Scene%20Component%20Object%20Reference))
  (bind _charactermeshother (Variables|Default|GetCharacterMeshOther))
  (Collision|SetCollisionProfileName (Variables|Default|GetCapsuleComponent) "NoCollision" true :!class /Script/Engine.PrimitiveComponent)
  (Collision|SetCollisionProfileName (Variables|Character|GetMesh) "Ragdoll" true :!class /Script/Engine.PrimitiveComponent)
  (Collision|SetCollisionResponsetoChannel (Variables|Character|GetMesh) "ECC_Visibility" "ECR_Block")
  (Development|SetHiddeninGame (Variables|Default|GetCharacterMeshOther) false false)
  (Components|SkinnedMesh|HideBonebyName (Variables|Character|GetMesh) "spine_01" "PBO_None")
  (Components|SkinnedMesh|HideBonebyName _charactermeshother "thigh_l" "PBO_None")
  (Components|SkinnedMesh|HideBonebyName _charactermeshother "thigh_r" "PBO_None")
  (Physics|AddImpulse _charactermeshother "600.000000,600.000000,12000.000000" "spine_01" true)
  (Niagara|SpawnSystematLocation "/Game/Core/VFX/Blood/NS_Blood.NS_Blood" (Transformation|GetSocketLocation (Variables|Character|GetMesh) "spine_01") (Math|Rotator|MakeRotfromZ (Transformation|GetComponentVelocity ServerSawblade))))

(event Custom|ServerSetCurrentScale
  (params (ServerCurrentScale :type Vector))
  (Variables|/Game/Core/ShrinkGrow/AC_ShrinkGrowActor.AC_ShrinkGrowActor_C|SetCurrentScale (Variables|Default|GetAC_ShrinkGrowActor) ServerCurrentScale))

(event EventSlice
  (params (SawMesh :type Scene%20Component%20Object%20Reference))
  (CallFunction|ServerSliceEffect SawMesh))

(event EventSetCurrentScale
  (params (ActorCurrentScale :type Vector :default "0, 0, 0"))
  (CallFunction|ServerSetCurrentScale ActorCurrentScale))

(fn ConstructionScript)