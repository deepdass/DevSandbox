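; BP_PhysicsCube is an interactive cube that gets a random color and can be sliced by a saw mesh.
; Construction copies the static cube into a procedural mesh with collision so it can be cut at runtime.
; The authority picks a random saturated hue on BeginPlay, and an OnRep applies it to the material.
; Slice cuts along the saw's plane, caps the cut, then launches the resulting piece with physics and an impulse.
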(event Custom|SetCubeColor
  (params (Color :type Linear%20Color%20Structure))
  (Rendering|Material|SetVectorParameterValueonMaterials (Variables|Default|GetProceduralMesh) "BaseColor" (Math|Conversions|ToVector(LinearColor) Color)))

(event EventBeginPlay
  (if (Ability|HasAuthority)
    (bind _output_get (Variables|Default|SetCubeColor (Class|KismetMathLibrary|HSVtoRGB (Math|Random|RandomFloatinRange 0.0 3.6e+02) 1.0 1.0 1.0)))
    (CallFunction|SetCubeColor _output_get)))

(event EventSlice
  (params (SawMesh :type Scene%20Component%20Object%20Reference))
  (bind _outotherhalfprocmesh (Class|KismetProceduralMeshLibrary|SliceProceduralMesh (Variables|Default|GetProceduralMesh) (Transformation|GetWorldLocation SawMesh) (Math|Vector|GetUpVector SawMesh) true "CreateNewSectionForCap" "/AnimationSharing/AnimSharingRed.AnimSharingRed"))
  (Physics|SetSimulatePhysics _outotherhalfprocmesh true)
  (Physics|AddImpulse _outotherhalfprocmesh "400.000000,400.000000,400.000000" "None" true))

(fn ConstructionScript
  (Class|KismetProceduralMeshLibrary|CopyProceduralMeshfromStaticMeshComponent (Variables|Default|GetCube) 0 (Variables|Default|GetProceduralMesh) true))

(fn OnRepCubeColor
  (CallFunction|SetCubeColor (Variables|Default|GetCubeColor)))